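; BP_LevelSpawner populates a level with a configurable number of enemies of a chosen type when play begins.
; Each spawn point is random within Y and Z bounds at zero X, then shifted by an offset, placing enemies on a single plane.
; Positions are in world space, independent of the spawner's own transform, and spawning ignores collisions.
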(event EventBeginPlay
  (bind _spawnbounds (Variables|Default|GetSpawnBounds))
  (bind (_x _y _z) (Math|Vector|BreakVector _spawnbounds))
  (for _index (range 0 (Variables|Default|GetSpawnCount))
    (Game|SpawnActorfromClass (Variables|Default|GetEnemyType) (Math|Transform|MakeTransform (+ (Math|Vector|MakeVector 0.0 (Math|Random|RandomFloatinRange (* _y -1.0) _y) (Math|Random|RandomFloatinRange (* _z -1.0) _z)) (Variables|Default|GetSpawnOffset))) "AlwaysSpawn" 0 0)))

(fn ConstructionScript)