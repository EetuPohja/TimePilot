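; Player pawn that flies in a vertical plane using FloatingPawnMovement, with engine thrust and twin guns.
; Tick feeds left-stick input into movement, scales engine trail spawning by thrust, and rolls the mesh toward the stick, or toward velocity when idle.
; The controller's thrust event plays a timeline that drives TurningBoost.
; Firing creates a gun component that a looping timer fires from both hand sockets; stopping destroys it.
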(event Custom|OnThrust
  (bind _boost_amount (Timeline|OnThrustBoost PlayFromStart)
    (:Update
      (Variables|/Script/Engine.FloatingPawnMovement|SetTurningBoost (Variables|Default|GetFloatingPawnMovement) _boost_amount))))

(event Custom|FireActiveGun
  (Class|WeaponBase|Fire (Variables|Default|GetActiveGun) (Transformation|GetSocketTransform (Variables|Default|GetSkeletalMesh) "Socket_Gun_R" "RTS_World"))
  (Class|WeaponBase|Fire (Variables|Default|GetActiveGun) (Transformation|GetSocketTransform (Variables|Default|GetSkeletalMesh) "Socket_Gun_L" "RTS_World")))

(event EventBeginPlay
  (bind _returnvalue (Game|GetPlayerController 0))
  (bind _self self)
  (Game|Player|SetViewTargetwithBlend _returnvalue _self 0.0 "VTBlend_Linear" 0.0 false)
  (Input|EnableInput _self _returnvalue)
  (bind _astp2k_player_controller (Utilities|Casting|CastToTP2K_PlayerController (Game|GetPlayerController 0)))
  (EventDispatchers|BindEventtoOnPlayerThrust _astp2k_player_controller (delegate Custom|OnThrust)))

(event EventStartFireGun
  (bind _returnvalue (Game|AddComponentbyClass (Utilities|Array|Get(acopy) (Variables|Default|Getm_aGuns))))
  (bind _output_get (Variables|Default|SetActiveGun _returnvalue))
  (bind _returnvalue_2 (Utilities|Time|SetTimerbyEvent (delegate Custom|FireActiveGun) (.fFireDelay (Utilities|Struct|BreakWeaponProperties (Class|WeaponBase|GetWeaponProperties _output_get))) true))
  (Variables|Default|SetGunTimerHandle _returnvalue_2)
  (CallFunction|FireActiveGun))

(event EventTick
  (params (DeltaSeconds :type Float%20%28single-precision%29))
  (bind _returnvalue (Game|GetPlayerController 0))
  (bind _floatingpawnmovement (Variables|Default|GetFloatingPawnMovement))
  (bind _meshparent (Variables|Default|GetMeshParent))
  (bind _returnvalue_2 (Transformation|GetWorldRotation _meshparent))
  (bind _velocity (Variables|/Script/Engine.MovementComponent|GetVelocity _floatingpawnmovement))
  (bind _returnvalue_3 (Math|Vector|VectorLength _velocity))
  (bind _returnvalue_4 (Math|Rotator|MakeRotfromX _velocity))
  (bind _returnvalue_5 (> _returnvalue_3 0.01))
  (bind _returnvalue_6 (+ (.pitch _returnvalue_4) -9e+01))
  (bind _astp2k_player_controller (Utilities|Casting|CastToTP2K_PlayerController _returnvalue))
  (Effects|Components|ParticleSystem|SetFloatParameter (Variables|Default|GetEngineTrail) "UserSpawnRate" (* (Class|TP2KPlayerController|GetThrustValue _astp2k_player_controller) 5e+02))
  (bind _asbp_player_controller (Utilities|Casting|CastToBP_PlayerController _returnvalue))
  (Pawn|Input|AddMovementInput (Transformation|GetActorRightVector) (.X (Math|Vector|BreakVector (Class|TP2KPlayerController|GetLeftStickScaled _asbp_player_controller))) false)
  (Pawn|Input|AddMovementInput (Transformation|GetActorUpVector) (.Y (Math|Vector|BreakVector (Class|TP2KPlayerController|GetLeftStickScaled _asbp_player_controller))) false)
  (if (Math|Float|NearlyEqual(Float) (Math|Vector|VectorLength (Class|TP2KPlayerController|GetLeftStickScaled _asbp_player_controller)) 0.0 0.0001)
    (if (> (.Y (Math|Vector|BreakVector _velocity)) 0.0)
      (if _returnvalue_5
        (Transformation|SetRelativeRotation _meshparent (Math|Interpolation|RInterpTo _returnvalue_2 (Math|Rotator|MakeRotator (* _returnvalue_6 -1.0) 0.0 0.0) DeltaSeconds 2.0) false false))
      (elif _returnvalue_5
        (Transformation|SetRelativeRotation _meshparent (Math|Interpolation|RInterpTo _returnvalue_2 (Math|Rotator|MakeRotator _returnvalue_6 0.0 0.0) DeltaSeconds 2.0) false false)))
    (else
      (Transformation|SetRelativeRotation _meshparent (Math|Interpolation|RInterpTo _returnvalue_2 (Math|Rotator|MakeRotator (+ (.yaw (Class|KismetMathLibrary|NegateRotator (Math|Rotator|MakeRotfromX (Class|TP2KPlayerController|GetLeftStickScaled _asbp_player_controller)))) 9e+01) 0.0 0.0) DeltaSeconds 8.0) false false))))

(event EventStopFireGun
  (bind _activegun (Variables|Default|GetActiveGun))
  (Utilities|Time|ClearandInvalidateTimerbyHandle (Variables|Default|GetGunTimerHandle))
  (Utilities|IsValid _activegun
    (:Is%20Valid
      (Components|DestroyComponent _activegun))))

(fn ConstructionScript)