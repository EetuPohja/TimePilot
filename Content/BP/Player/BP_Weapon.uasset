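; BP_Weapon is a player weapon that spawns projectiles from a socket transform when its Fire event runs.
; The weapon properties struct supplies the projectile class and the bullets-per-shot count that drives the spawn loop.
; Each spawned BP_BasicProjectile receives the socket's forward vector, without spread, plus the velocity of player pawn 0, its owner and instigator.
; The fire sound plays at the socket once per projectile.
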(event EventBeginPlay)

(event EventTick
  (params (DeltaSeconds :type Float%20%28single-precision%29)))

(event EventFire
  (params (SocketTransform :type Transform%20%28by%20ref%29))
  (bind (_location _rotation) (Math|Transform|BreakTransform SocketTransform))
  (bind _returnvalue (Game|Player|GetPlayerPawn 0))
  (bind _m_weaponproperties (Variables|Default|Getm_WeaponProperties))
  (bind (_fbulletspershot _pprojectile) (Utilities|Struct|BreakWeaponProperties _m_weaponproperties))
  (for _index (range 0 (Math|Float|Truncate _fbulletspershot))
    (bind _returnvalue_2 (Game|SpawnActorfromClass _pprojectile (Math|Transform|MakeTransform _location) "Undefined" _returnvalue _returnvalue))
    (bind _asbp_basic_projectile (Utilities|Casting|CastToBP_BasicProjectile _returnvalue_2))
    (Utilities|IsValid _asbp_basic_projectile
      (:Is%20Valid
        (Class|ProjectileBase|SetupProjectile _asbp_basic_projectile (Math|Rotator|GetRotationXVector _rotation) (Transformation|GetVelocity _returnvalue))
        (Audio|PlaySoundatLocation (Variables|Default|GetFX) _location "0, 0, 0" 1.0 1.0 0.0 0 0 0)))))